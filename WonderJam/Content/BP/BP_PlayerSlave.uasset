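; Player-controlled racer pawn that auto-runs along a referenced spline, with one of six character profiles chosen by the Game Instance's IdEsclave.
; BeginPlay applies that profile's mesh, name, speed, endurance drain and obedience, then starts a timeline that moves and rotates the actor along the spline.
; A looping timer drains Endurance, retiming the timeline's play rate from spline length, speed and endurance.
; SetVitesse and SetTime let speed or duration change mid-run.
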(event `self.ReceiveBeginPlay`
  (bind _returnvalue (`SplineComponent.GetSplineLength` (`/Game/BP/BP_Spline.Spline` (`self.Spline REF`))))
  (bind _returnvalue_2 (/ _returnvalue (* (`self.Vitesse`) (+ 1.0 (`self.Endurance`)))))
  (set `self.Endurance` 1.0)
  (`KismetSystemLibrary.K2_SetTimerDelegate` (delegate `CustomEvent`) 5.0 true)
  (`KismetSystemLibrary.PrintString` (`KismetStringLibrary.Conv_DoubleToString` _returnvalue) true true (struct :`G` 0.66 :`B` 1.0 :`A` 1.0) 20.0)
  (bind _asbp_gameinstance (cast `/Game/BP/BP_Gameinstance` (`GameplayStatics.GetGameInstance`)))
  (bind _idesclave (`/Game/BP/BP_Gameinstance.idEsclave` _asbp_gameinstance))
  (if (== _idesclave 0)
    (bind _output_get (set `self.New Mesh` "/Game/Charactere/character.character"))
    (set `self.name` "Pipo Bimbo")
    (set `self.Vitesse` 150.0)
    (set `self.EnduranceDecr` 0.03)
    (set `self.obeissance` 0.4)
    (`KismetSystemLibrary.PrintString` (`KismetStringLibrary.Conv_DoubleToString` _returnvalue_2) :!label _label)
    (set `self.Time to Complete ` _returnvalue_2)
    (`SkeletalMeshComponent.SetSkeletalMeshAsset` (`self.skeletal`) _output_get)
    (`self.Move Object`)
    (elif (== _idesclave 1)
      (set `self.New Mesh` "/Game/Charactere/character__1_.character__1_")
      (set `self.name` "Chen Zen")
      (set `self.Vitesse` 1300.0)
      (set `self.EnduranceDecr` 0.06)
      (set `self.obeissance` 1.0)
      (goto _label)
      (elif (== _idesclave 2)
        (set `self.New Mesh` "/Game/Charactere/character__2_.character__2_")
        (set `self.name` "Naps")
        (set `self.Vitesse` 110.0)
        (set `self.EnduranceDecr` 0.01)
        (set `self.obeissance` 0.6)
        (goto _label)
        (elif (== _idesclave 3)
          (set `self.New Mesh` "/Game/Charactere/character__3_.character__3_")
          (set `self.name` "Orelsan")
          (set `self.Vitesse` 150.0)
          (set `self.EnduranceDecr` 0.04)
          (set `self.obeissance` 0.6)
          (goto _label)
          (elif (== _idesclave 4)
            (set `self.New Mesh` "/Game/Charactere/character__4_.character__4_")
            (set `self.name` "Avatar")
            (set `self.Vitesse` 170.0)
            (set `self.EnduranceDecr` 0.03)
            (set `self.obeissance` 0.2)
            (goto _label)
            (elif (== _idesclave 5)
              (set `self.New Mesh` "/Game/Charactere/character__5_.character__5_")
              (set `self.name` "Hamilton")
              (set `self.Vitesse` 190.0)
              (set `self.EnduranceDecr` 0.06)
              (set `self.obeissance` 0.4)
              (goto _label))))))))

(event `CustomEvent`
  (`self.SetStamina` (`self.EnduranceDecr`))
  (`KismetSystemLibrary.PrintString` (`KismetStringLibrary.Conv_DoubleToString` (`self.Endurance`)))
  (`KismetSystemLibrary.PrintString` (`KismetStringLibrary.Conv_DoubleToString` (`self.EnduranceDecr`))))

(event `Move Object`
  (bind _spline (`/Game/BP/BP_Spline.Spline` (`self.Spline REF`)))
  (`TimelineComponent.SetPlayRate` (`self.Move object T`) (/ 1.0 (`self.Time to Complete `)))
  (bind (_direction _move_track) (`Timeline|Move object T` :!via `PlayFromStart`)
    (:`Update`
      (bind _returnvalue (`KismetMathLibrary.Lerp` 0.0 (`SplineComponent.GetSplineLength` (`/Game/BP/BP_Spline.Spline` (`self.Spline REF`))) _move_track))
      (`self.K2_SetActorTransform` (`KismetMathLibrary.MakeTransform` (`SplineComponent.GetLocationAtDistanceAlongSpline` _spline _returnvalue "World") (`SplineComponent.GetRotationAtDistanceAlongSpline` _spline _returnvalue "Local"))))))

(event `SetTime`
  (params (Timetocomplete :type "Float (double-precision)"))
  (bind _move_object_t (`self.Move object T`))
  (`TimelineComponent.Stop` _move_object_t)
  (`TimelineComponent.SetPlayRate` _move_object_t (/ 1.0 Timetocomplete))
  (`TimelineComponent.Play` _move_object_t))

(event `SetStamina`
  (params (Decrease :type "Float (double-precision)"))
  (bind _move_object_t (`self.Move object T`))
  (if (not (<= (`self.Endurance`) 0.0))
    (bind _output_get (set `self.Endurance` (- (`self.Endurance`) Decrease)))
    (`TimelineComponent.Stop` _move_object_t)
    (`TimelineComponent.SetPlayRate` _move_object_t (/ 1.0 (/ (`SplineComponent.GetSplineLength` (`/Game/BP/BP_Spline.Spline` (`self.Spline REF`))) (* (`self.Vitesse`) (+ 1.0 _output_get)))))
    (`TimelineComponent.Play` _move_object_t)))

(event `SetVitesse`
  (params (value :type "Float (double-precision)"))
  (bind _move_object_t (`self.Move object T`))
  (bind _output_get (set `self.Vitesse` (+ value (`self.Vitesse`))))
  (`TimelineComponent.Stop` _move_object_t)
  (`TimelineComponent.SetPlayRate` _move_object_t (/ 1.0 (/ (`SplineComponent.GetSplineLength` (`/Game/BP/BP_Spline.Spline` (`self.Spline REF`))) (* _output_get (+ 1.0 (`self.Endurance`))))))
  (`TimelineComponent.Play` _move_object_t)
  (`KismetSystemLibrary.PrintString` (`KismetStringLibrary.Conv_DoubleToString` (`self.Vitesse`))))

(fn `UserConstructionScript`)