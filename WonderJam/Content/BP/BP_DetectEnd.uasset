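; BP_DetectEnd is an overlap trigger that tallies finish passes for the player slave versus other actors, likely as a race end line.
; Each overlap event loops over all overlapping actors and increments one of two counters, matching the player by the hard-coded object name BP_PlayerSlave_C_1.
; When either counter equals four, it only prints a finish message, alongside debug prints.
; BeginPlay resets just the player counter.
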(event `self.ReceiveBeginPlay`
  (set `self.finish_player` 0))

(event `self.ReceiveActorBeginOverlap`
  (params (OtherActor :type "Actor Object Reference"))
  (for _array_element (`self.GetOverlappingActors` null)
    (bind _returnvalue (`KismetSystemLibrary.GetObjectName` _array_element))
    (`KismetSystemLibrary.PrintString` _returnvalue)
    (if (`KismetStringLibrary.EqualEqual_StrStr` "BP_PlayerSlave_C_1" _returnvalue)
      (`KismetSystemLibrary.PrintString` "okay")
      (`/Engine/EditorBlueprintResources/StandardMacros.IncrementInt` (`self.finish_player`)
        (:`  `
          (if (== 4 (`self.finish_player`))
            (`KismetSystemLibrary.PrintString` "Slave finish youhou"))))
      (else
        (`KismetSystemLibrary.PrintString` "false")
        (`/Engine/EditorBlueprintResources/StandardMacros.IncrementInt` (`self.finsih_other`)
          (:`  `
            (if (== 4 (`self.finsih_other`))
              (`KismetSystemLibrary.PrintString` "Other finish :("))))))))

(fn `UserConstructionScript`)