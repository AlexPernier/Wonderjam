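; BP_SphereRun3 is an actor that travels along a referenced spline, starting at BeginPlay.
; It destroys itself instead when the BP_Gameinstance IdEsclave is 3, and does nothing if that cast fails.
; A timeline, rate-scaled by the inverse of TimeToComplete, maps its track to distance along the spline.
; Each update sets location in world space but rotation in the spline's local space.
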(event `self.ReceiveBeginPlay`
  (bind _asbp_gameinstance (cast `/Game/BP/BP_Gameinstance` (`GameplayStatics.GetGameInstance`)))
  (if (== 3 (`/Game/BP/BP_Gameinstance.idEsclave` _asbp_gameinstance))
    (`self.K2_DestroyActor`)
    (else
      (`self.Move Object`))))

(event `Move Object`
  (bind _spline (`/Game/BP/BP_Spline.Spline` (`self.Spline REF`)))
  (`TimelineComponent.SetPlayRate` (`self.Move object T`) (/ 1.0 (`self.Time to Complete `)))
  (bind (_direction _move_track) (`Timeline|Move object T`)
    (:`Update`
      (bind _returnvalue (`KismetMathLibrary.Lerp` 0.0 (`SplineComponent.GetSplineLength` (`/Game/BP/BP_Spline.Spline` (`self.Spline REF`))) _move_track))
      (`self.K2_SetActorTransform` (`KismetMathLibrary.MakeTransform` (`SplineComponent.GetLocationAtDistanceAlongSpline` _spline _returnvalue "World") (`SplineComponent.GetRotationAtDistanceAlongSpline` _spline _returnvalue "Local"))))))

(fn `UserConstructionScript`)